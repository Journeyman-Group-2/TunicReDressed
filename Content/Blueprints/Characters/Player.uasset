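; Player character Blueprint that handles movement input, item interaction input and on-screen UI.
; Forward and right axes move it along the control yaw only, while turn-rate and look-up-rate axis events are unwired.
; Pickup, Use and Drop inputs set flags on PickupComponent, and Run starts or ends running through StaminaComponent.
; BeginPlay adds the main UI and a hidden pickup prompt widget to the viewport.
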(event `self.ReceiveBeginPlay`
  (`parent.ReceiveBeginPlay`)
  (`self.InitializeUI`))

(event `InputAxis|TurnRate`
  (params (AxisValue :type "Float (single-precision)"))
  ;[1 1 1] Controller Rotation Input
)

(event `InputAxis|LookUpRate`
  (params (AxisValue :type "Float (single-precision)"))
  ;[1 1 1] Controller Rotation Input
)

(event `self.ReceiveTick`
  (params (DeltaSeconds :type "Float (single-precision)"))
  ;[1 1 1] Tick
  (`parent.ReceiveTick` DeltaSeconds))

(event `InputAxis|MoveForward` :overrideparent false
  (params (AxisValue :type "Float (single-precision)"))
  ;[1 1 1] Character Movement Rotation
  (`self.AddMovementInput` (`KismetMathLibrary.GetForwardVector` (`KismetMathLibrary.MakeRotator` 0.0 0.0 (.yaw (`self.GetControlRotation`)))) AxisValue))

(event `InputAxis|MoveRight` :overrideparent false
  (params (AxisValue :type "Float (single-precision)"))
  ;[1 1 1] Character Movement Rotation
  (`self.AddMovementInput` (`KismetMathLibrary.GetRightVector` (`KismetMathLibrary.MakeRotator` 0.0 0.0 (.yaw (`self.GetControlRotation`)))) AxisValue))

(event `InputAction|Pickup`
  (params (Key :type "Key Structure"))
  (bind _pickupcomponent (`self.PickupComponent`))
  ;[1 1 1] Action Mappings Keyboard
  (:`Pressed`
    (set `/Game/Blueprints/CharacterBaseWithComponents/PickupComponent.TryingToPickup` true _pickupcomponent))
  (:`Released`
    (set `/Game/Blueprints/CharacterBaseWithComponents/PickupComponent.TryingToPickup` false _pickupcomponent)))

(event `InputAction|Use`
  (params (Key :type "Key Structure"))
  (bind _pickupcomponent (`self.PickupComponent`))
  ;[1 1 1] Action Mappings Keyboard
  (:`Pressed`
    (set `/Game/Blueprints/CharacterBaseWithComponents/PickupComponent.TryingToUse` true _pickupcomponent))
  (:`Released`
    (set `/Game/Blueprints/CharacterBaseWithComponents/PickupComponent.TryingToUse` false _pickupcomponent)))

(event `InputAction|Run`
  (params (Key :type "Key Structure"))
  (bind _staminacomponent (`self.StaminaComponent`))
  ;[1 1 1] Action Mappings Keyboard
  (:`Pressed`
    (`/Game/Blueprints/CharacterBaseWithComponents/StaminaComponent.BeginRun` _staminacomponent))
  (:`Released`
    (`/Game/Blueprints/CharacterBaseWithComponents/StaminaComponent.End Run` _staminacomponent)))

(event `InputAction|Drop`
  (params (Key :type "Key Structure"))
  (bind _pickupcomponent (`self.PickupComponent`))
  ;[1 1 1] Action Mappings Keyboard
  (:`Pressed`
    (set `/Game/Blueprints/CharacterBaseWithComponents/PickupComponent.DropItem` true _pickupcomponent))
  (:`Released`
    (set `/Game/Blueprints/CharacterBaseWithComponents/PickupComponent.DropItem` false _pickupcomponent)))

(fn `InitializeUI`
  ;[1 1 1] Begin Play
  (bind _returnvalue (`|CreateWidget` "/Game/Blueprints/UI/UI.UI_C"))
  (set `self.UI` _returnvalue)
  (`UserWidget.AddToViewport` _returnvalue 0)
  (bind _returnvalue_2 (`|CreateWidget` "/Game/Blueprints/UI/PickUpUI.PickUpUI_C"))
  (bind _output_get (set `self.PickupUI` _returnvalue_2))
  (`Widget.SetVisibility` _output_get "Hidden")
  (`UserWidget.AddToViewport` _output_get 0))

(fn `UserConstructionScript`
  (`parent.UserConstructionScript`))