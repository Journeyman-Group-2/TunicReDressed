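; Camera focus component that shifts the player's spring arm and camera to a combat framing when a living AI enemy is near.
; Each tick it finds the closest AI within range and toggles between default and focus presets, returning when that enemy dies or leaves.
; Transitions lerp camera transform and arm length over time.
; Before focusing, it offsets the focus yaw by the clamped player-to-target angle from a dot product.
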(event `self.ReceiveBeginPlay`
  (bind _returnvalue (`GameplayStatics.GetPlayerCharacter` 0))
  (bind _focusarray (`self.FocusArray`))
  (set `self.ActorRef` _returnvalue)
  (set `self.SpringArm` (`Actor.GetComponentByClass` _returnvalue "/Script/Engine.SpringArmComponent"))
  (set `self.Camera` (`Actor.GetComponentByClass` _returnvalue "/Script/Engine.CameraComponent"))
  (`KismetArrayLibrary.Array_Set` _focusarray 0 (make `/Game/Blueprints/Characters/Focus` (`SpringArmComponent.TargetArmLength` (`self.SpringArm`)) (`SceneComponent.GetRelativeTransform` (`self.Camera`))))
  (set `self.previousFocus2` (`|GetArrayItem` _focusarray 1)))

(event `self.ReceiveTick`
  (params (DeltaSeconds :type "Float (single-precision)"))
  (`self.UpdateCameraFocusCycle`)
  (`self.UpdateSpringArmFocus` DeltaSeconds))

(fn `SetTransformYawBasedOnTargetPoint`
  (bind _output (`|GetArrayItem` (`self.FocusArray`)))
  (bind _output_2 (`|GetArrayItem` (`self.FocusArray`) 1))
  (bind _output_3 (`|GetArrayItem` (`self.FocusArray`) 1))
  (bind (_returnvalue_x _returnvalue_y _returnvalue_z) (`KismetMathLibrary.BreakVector` (`KismetMathLibrary.Normal` (- (`self.targetPoint`) (.location (`.CameraTransform_8_A9FA57204E52756CC7AFEFA74F9966B6` (break `/Game/Blueprints/Characters/Focus` _output)))))))
  (bind (_returnvalue_x_2 _returnvalue_y_2 _returnvalue_z_2) (`KismetMathLibrary.BreakVector` (`KismetMathLibrary.Normal` (- (`Actor.K2_GetActorLocation` (`self.ActorRef`)) (.location (`.CameraTransform_8_A9FA57204E52756CC7AFEFA74F9966B6` (break `/Game/Blueprints/Characters/Focus` _output)))))))
  (bind _returnvalue (`KismetMathLibrary.FClamp` (`KismetMathLibrary.DegAcos` (`KismetMathLibrary.Dot_VectorVector` (`KismetMathLibrary.MakeVector` _returnvalue_x_2 _returnvalue_y_2 _returnvalue_z_2) (`KismetMathLibrary.MakeVector` _returnvalue_x _returnvalue_y _returnvalue_z))) 0.0 (`self.MaxDeltaYaw`)))
  (if (== (`self.FocusIndex`) 0)
    (`KismetArrayLibrary.Array_Set` (`self.FocusArray`) 1 (`self.previousFocus2`)) ; reset 2nd transform
    (if (> _returnvalue_x _returnvalue_x_2)
      ;[1 1 1] Comment
      (`KismetArrayLibrary.Array_Set` (`self.FocusArray`) 1 (make `/Game/Blueprints/Characters/Focus` (break `/Game/Blueprints/Characters/Focus` _output_3) (`KismetMathLibrary.MakeTransform` (.location (`.CameraTransform_8_A9FA57204E52756CC7AFEFA74F9966B6` (break `/Game/Blueprints/Characters/Focus` _output_3))) (`KismetMathLibrary.MakeRotator` (.roll (.rotation (`.CameraTransform_8_A9FA57204E52756CC7AFEFA74F9966B6` (break `/Game/Blueprints/Characters/Focus` _output_3)))) (.pitch (.rotation (`.CameraTransform_8_A9FA57204E52756CC7AFEFA74F9966B6` (break `/Game/Blueprints/Characters/Focus` _output_3)))) (+ (.yaw (.rotation (`.CameraTransform_8_A9FA57204E52756CC7AFEFA74F9966B6` (break `/Game/Blueprints/Characters/Focus` _output_3)))) _returnvalue)) (.scale (`.CameraTransform_8_A9FA57204E52756CC7AFEFA74F9966B6` (break `/Game/Blueprints/Characters/Focus` _output_3))))))
      (else
        ;[1 1 1] Comment
        (`KismetArrayLibrary.Array_Set` (`self.FocusArray`) 1 (make `/Game/Blueprints/Characters/Focus` (break `/Game/Blueprints/Characters/Focus` _output_2) (`KismetMathLibrary.MakeTransform` (.location (`.CameraTransform_8_A9FA57204E52756CC7AFEFA74F9966B6` (break `/Game/Blueprints/Characters/Focus` _output_2))) (`KismetMathLibrary.MakeRotator` (.roll (.rotation (`.CameraTransform_8_A9FA57204E52756CC7AFEFA74F9966B6` (break `/Game/Blueprints/Characters/Focus` _output_2)))) (.pitch (.rotation (`.CameraTransform_8_A9FA57204E52756CC7AFEFA74F9966B6` (break `/Game/Blueprints/Characters/Focus` _output_2)))) (- (.yaw (.rotation (`.CameraTransform_8_A9FA57204E52756CC7AFEFA74F9966B6` (break `/Game/Blueprints/Characters/Focus` _output_2)))) _returnvalue)) (.scale (`.CameraTransform_8_A9FA57204E52756CC7AFEFA74F9966B6` (break `/Game/Blueprints/Characters/Focus` _output_2))))))))))

(fn `UpdateCameraFocusCycle`
  (bind _returnvalue (> (`self.FocusIndex`) 0))
  (if (not (`self.isFocusingActive`))
    (bind _updatesucceeded (`self.UpdateTargetPoint`)) ; get a target enemy
    (if _updatesucceeded
      (bind _outactors (`GameplayStatics.GetAllActorsOfClass` "/Game/Blueprints/Characters/AI.AI_C"))
      (bind _health (`/Game/Blueprints/CharacterBaseWithComponents/HealthComponent.GetHealth` (`/Game/Blueprints/CharacterBaseWithComponents/CharacterComponents.HealthComponent` (`|GetArrayItem` _outactors (`self.ClosestAiIndex`)))))
      (if (> _health 0.0)
        (if (== (`self.FocusIndex`) 0)
          (set `self.isFocusingActive` true :!label _label)
          (`self.SetTransformYawBasedOnTargetPoint`))
        (elif _returnvalue
          (goto _label)))
      (elif _returnvalue
        (goto _label)))))

(fn `UpdateSpringArmFocus`
  (params (DeltaTime :type "Float (double-precision)"))
  (bind (_output_targetarmlength _output_cameratransform) (break `/Game/Blueprints/Characters/Focus` (`|GetArrayItem` (`self.FocusArray`) (`self.FocusIndex`))))
  (bind _returnvalue (mod (+ (`self.FocusIndex`) 1) (`KismetArrayLibrary.Array_Length` (`self.FocusArray`))))
  (bind _returnvalue_2 (`KismetMathLibrary.FClamp` (/ (`self.currentTimeToFocus`) (`self.timeToFocus`))))
  (bind (_output_targetarmlength_2 _output_cameratransform_2) (break `/Game/Blueprints/Characters/Focus` (`|GetArrayItem` (`self.FocusArray`) _returnvalue)))
  (if (`self.isFocusingActive`)
    (set `self.currentTimeToFocus` (+ (`self.currentTimeToFocus`) DeltaTime))
    (if (== _returnvalue_2 1.0)
      (set `self.isFocusingActive` false)
      (set `self.currentTimeToFocus` 0.0)
      (set `self.FocusIndex` _returnvalue))
    (`SceneComponent.K2_SetRelativeTransform` (`self.Camera`) (`KismetMathLibrary.TLerp` _output_cameratransform _output_cameratransform_2 _returnvalue_2) false false)
    (set `SpringArmComponent.TargetArmLength` (`KismetMathLibrary.Lerp` _output_targetarmlength _output_targetarmlength_2 _returnvalue_2) (`self.SpringArm`))))

(fn `UpdateTargetPoint`
  (returns (UpdateSucceeded :type Boolean))
  (bind _returnvalue (`Actor.K2_GetActorLocation` (`self.ActorRef`)))
  ;[1 1 1] Get and validate enemies
  (bind _outactors (`GameplayStatics.GetAllActorsOfClass` "/Game/Blueprints/Characters/AI.AI_C")) ; get all enemies
  (if (> (`KismetArrayLibrary.Array_Length` _outactors) 0)
    (set `self.ClosestAiIndex` 0) ; index avaliable, 0 is first
    ;[1 1 1] Loop through each enemy and set the closest one's index
    (for (_ _array_index) _outactors
      (if (!= _array_index 0)
        (if (< (`KismetMathLibrary.Vector_Distance` (`Actor.K2_GetActorLocation` (`|GetArrayItem` _outactors _array_index)) _returnvalue) (`KismetMathLibrary.Vector_Distance` _returnvalue (`Actor.K2_GetActorLocation` (`|GetArrayItem` _outactors (`self.ClosestAiIndex`)))))
          (set `self.ClosestAiIndex` _array_index))))
    ;[1 1 1] Validate closest enemy
    (bind _output_get (set `self.targetPoint` (`Actor.K2_GetActorLocation` (`|GetArrayItem` _outactors (`self.ClosestAiIndex`)))))
    (if (< (`KismetMathLibrary.Vector_Distance` _output_get (`Actor.K2_GetActorLocation` (`self.ActorRef`))) (`self.FocusWhenDistanceIsLessThen`))
      (return true)
      (else
        (return false)))
    (else
      (set `self.ClosestAiIndex` -1) ; no index avaliable
    )))