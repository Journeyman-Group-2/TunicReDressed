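; MannaComponent is a component that tracks a character's manna pool and regenerates it over time.
; Tick accumulates delta time and adds the regen amount once per elapsed interval, using a loop to catch up when several intervals pass in one frame.
; AddManna and UseManna clamp the value between zero and the maximum.
; Helper functions report the fill ratio and check whether a cost is affordable.
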(event `self.ReceiveBeginPlay`)

(event `self.ReceiveTick`
  (params (DeltaSeconds :type "Float (single-precision)"))
  (set `self.Time` (+ DeltaSeconds (`self.Time`)))
  (while (>= (`self.Time`) (`self.RegenEveryNSeconds`))
    (set `self.Time` (- (`self.Time`) (`self.RegenEveryNSeconds`)))
    (`self.AddManna` (`self.RegenAmount`))))

(fn `AddManna`
  (params (Manna :type Integer))
  (set `self.Manna` (`KismetMathLibrary.Clamp` (+ (`self.Manna`) Manna) 0 (`self.MaxManna`))))

(fn `CanUseManna`
  (params (Manna :type Integer))
  (returns (Result :type Boolean))
  (return (<= Manna (`self.Manna`))))

(fn `GetMannaPercentage`
  (returns (NewParam :type "Float (double-precision)"))
  (return (/ (`KismetMathLibrary.Conv_IntToDouble` (`self.Manna`)) (`KismetMathLibrary.Conv_IntToDouble` (`self.MaxManna`)))))

(fn `UseManna`
  (params (Manna :type Integer))
  (set `self.Manna` (`KismetMathLibrary.Clamp` (- (`self.Manna`) Manna) 0 (`self.MaxManna`))))