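; Actor component that lets a CharacterComponents character pick up, drop and use a collectable item.
; Each tick it checks input flags for those three actions.
; Pickup snaps the nearby collectable to the right hand socket using its stored in-hand transform and disables its collision.
; Dropping detaches it, restores collision and places it ahead of the character at capsule height, while use forwards delta time to the item.
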(event `self.ReceiveBeginPlay`
  (bind _returnvalue (`self.GetOwner`))
  ;[1 1 1] Begin Play
  (bind _ascharacter_components (cast `/Game/Blueprints/CharacterBaseWithComponents/CharacterComponents` _returnvalue))
  (set `self.Mesh` (`Actor.GetComponentByClass` _returnvalue "/Script/Engine.SkeletalMeshComponent"))
  (set `self.playerRef` _ascharacter_components))

(event `self.ReceiveTick`
  (params (DeltaSeconds :type "Float (single-precision)"))
  (`self.Update` DeltaSeconds))

(fn `Update`
  (params (DeltaTime :type "Float (double-precision)"))
  (bind _collectable (`self.Collectable`))
  (bind _mesh (`self.Mesh`))
  (bind _collectable_2 (`self.Collectable`))
  (bind (_transformwheninplayersrighthand_location _transformwheninplayersrighthand_rotation _transformwheninplayersrighthand_scale) (`KismetMathLibrary.BreakTransform` (`/Game/Blueprints/Weapons/Pickups/Base_PickupActor.TransformWhenInPlayersRightHand` _collectable_2)))
  (bind (_returnvalue_x _returnvalue_y _returnvalue_z) (`KismetMathLibrary.BreakVector` (`SceneComponent.K2_GetComponentLocation` (`Character.CapsuleComponent` (`self.playerRef`)))))
  (bind (_returnvalue_x_2 _returnvalue_y_2) (`KismetMathLibrary.BreakVector` (`SceneComponent.GetSocketLocation` _mesh (`SkinnedMeshComponent.GetSocketBoneName` _mesh "hand_r"))))
  (bind (_returnvalue_x_3 _returnvalue_y_3) (`KismetMathLibrary.BreakVector` (* (`SceneComponent.GetForwardVector` (`Actor.RootComponent` (`self.playerRef`))) 300.0)))
  (`|ExecutionSequence`
    (:`then_0`
      ;[1 1 1] Pickup
      (if (and (`self.TryingToPickup`) (`self.CanPickup`))
        (set `self.HasCollectable` true) ; set pickup
        (bind _output_get (set `self.Collectable` (`self.NearCollectable`))) ; set item
        (set `/Game/Blueprints/Weapons/Pickups/Base_PickupActor.PlayerRef` (`self.playerRef`) _output_get) ; set item player ref
        (`Actor.K2_AttachToComponent` _output_get (`self.Mesh`) "hand_r" "SnapToTarget" "SnapToTarget" "KeepRelative" true) ; attach item to player
        (`Actor.K2_SetActorRelativeTransform` _output_get (`KismetMathLibrary.MakeTransform` _transformwheninplayersrighthand_location _transformwheninplayersrighthand_rotation _transformwheninplayersrighthand_scale) false false) ; rotate item to fit in hand
        (`Actor.SetActorEnableCollision` _output_get false) ; turn off item collision
      ))
    (:`then_1`
      ;[1 1 1] Drop
      (if (`self.DropItem`)
        (if (`self.HasCollectable`)
          (set `self.HasCollectable` false)
          (`Actor.K2_DetachFromActor` _collectable "KeepWorld" "KeepWorld" "KeepWorld")
          (`Actor.SetActorEnableCollision` _collectable true)
          (`Actor.K2_SetActorTransform` _collectable_2 (`KismetMathLibrary.MakeTransform` (+ (`KismetMathLibrary.MakeVector` _returnvalue_x_2 _returnvalue_y_2 _returnvalue_z) (`KismetMathLibrary.MakeVector` _returnvalue_x_3 _returnvalue_y_3)) (struct) _transformwheninplayersrighthand_scale) false false)
          (`/Game/Blueprints/Weapons/Pickups/Base_PickupActor.LeaveBox` _collectable))))
    (:`then_2`
      ;[1 1 1] Use
      (if (and (`self.TryingToUse`) (`self.HasCollectable`))
        (`/Game/Blueprints/Weapons/Pickups/Base_PickupActor.Use` (`self.Collectable`) DeltaTime)))))