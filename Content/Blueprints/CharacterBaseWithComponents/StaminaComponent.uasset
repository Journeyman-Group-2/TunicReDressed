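; Stamina component for a CharacterComponents owner that powers a short, stamina-costing speed boost.
; BeginRun arms the boost if stamina suffices and no boost is running; EndRun clears the request.
; Tick starts one timed boost per request while moving, spending stamina and raising MaxWalkSpeed, and cuts it short when movement stops.
; Outside boosts, Tick restores normal speed and regenerates clamped stamina per frame, so recovery depends on frame rate.
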(event `self.ReceiveBeginPlay`
  ;[1 1 1] Event Begin Play
  (bind _ascharacter_components (cast `/Game/Blueprints/CharacterBaseWithComponents/CharacterComponents` (`self.GetOwner`)))
  (set `self.CharacterComponents` _ascharacter_components))

(event `self.ReceiveTick`
  (params (DeltaSeconds :type "Float (single-precision)"))
  (bind _charactercomponents (`self.CharacterComponents`))
  (bind _charactermovement (`Character.CharacterMovement` _charactercomponents))
  (bind _returnvalue (> (`KismetMathLibrary.VSize` (`CharacterMovementComponent.GetLastUpdateVelocity` (`Character.CharacterMovement` (`self.CharacterComponents`)))) 0.0))
  ;[1 1 1] Event Tick
  (if (`KismetSystemLibrary.IsValid` _charactercomponents)
    (if (<= (`self.SpeedBoostTime`) 0.0)
      (set `self.SpeedBoostTime` 0.0)
      (if (and (`self.RunBoost`) (not (`self.OnBoostCycle`)))
        (if _returnvalue
          (set `self.OnBoostCycle` true)
          (`self.ReduceStamina` (`self.StaminaNeededToBoost`))
          (set `CharacterMovementComponent.MaxWalkSpeed` 6000.0 _charactermovement)
          (set `self.SpeedBoostTime` (`self.SpeedBoostTimeReset`))
          (else
            (set `CharacterMovementComponent.MaxWalkSpeed` 600.0 _charactermovement :!label _label)
            (`self.IncreaseStamina` 1)))
        (else
          (goto _label)))
      (else
        (set `self.SpeedBoostTime` (- (`self.SpeedBoostTime`) DeltaSeconds))
        (if (not _returnvalue)
          (set `self.SpeedBoostTime` 0.0)
          (goto _label))))))

(fn `BeginRun`
  (if (>= (`self.Stamina`) (`self.StaminaNeededToBoost`))
    (if (== (`self.SpeedBoostTime`) 0.0)
      (set `self.RunBoost` true)
      (set `self.OnBoostCycle` false))))

(fn `End Run`
  (set `self.RunBoost` false)
  (set `self.OnBoostCycle` false))

(fn `GetStamina`
  (returns (NewParam :type Integer))
  (return (`self.Stamina`)))

(fn `GetStaminaPercentage`
  (returns (HealthPercentage :type "Float (double-precision)"))
  (return (/ (`KismetMathLibrary.Conv_IntToDouble` (`self.Stamina`)) (`KismetMathLibrary.Conv_IntToDouble` (`self.MaxStamina`)))))

(fn `IncreaseStamina`
  (params (Stamina :type Integer))
  (set `self.Stamina` (`KismetMathLibrary.Clamp` (+ (`self.Stamina`) Stamina) 0 (`self.MaxStamina`))))

(fn `ReduceStamina`
  (params (Stamina :type Integer))
  (set `self.Stamina` (`KismetMathLibrary.Clamp` (- (`self.Stamina`) Stamina) 0 (`self.MaxStamina`))))