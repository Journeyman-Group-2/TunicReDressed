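; Character base Blueprint built on components, handling death for characters, including the Player subclass.
; Tick polls HealthComponent, and at zero health or below it makes PickupComponent drop its item and turns the mesh into a physics ragdoll.
; After a short delay it removes the pickup and main UI if the character is a Player, then destroys the actor.
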(event `self.ReceiveBeginPlay`)

(event `self.ReceiveTick`
  (params (DeltaSeconds :type "Float (single-precision)"))
  (bind _pickupcomponent (`self.PickupComponent`))
  (bind _mesh (`self.Mesh`))
  (bind _health (`/Game/Blueprints/CharacterBaseWithComponents/HealthComponent.GetHealth` (`self.HealthComponent`)))
  (if (<= _health 0.0)
    (set `/Game/Blueprints/CharacterBaseWithComponents/PickupComponent.DropItem` true _pickupcomponent)
    (`/Game/Blueprints/CharacterBaseWithComponents/PickupComponent.Update` _pickupcomponent 0.0)
    (`SkeletalMeshComponent.SetAllBodiesSimulatePhysics` _mesh true)
    (`PrimitiveComponent.SetSimulatePhysics` _mesh true)
    (`PrimitiveComponent.WakeAllRigidBodies` _mesh)
    (`KismetSystemLibrary.Delay` 3.0)
    (bind _asplayer (cast `/Game/Blueprints/Characters/Player` self)
      (:`then`
        (`Widget.RemoveFromParent` (`/Game/Blueprints/Characters/Player.PickupUI` _asplayer))
        (`Widget.RemoveFromParent` (`/Game/Blueprints/Characters/Player.UI` _asplayer)))
      (:`CastFailed`
        _))
    (`self.K2_DestroyActor`)))

(fn `UserConstructionScript`)