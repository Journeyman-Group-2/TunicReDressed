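; Health component that tracks integer health against a maximum, apparently for the component-based character setup.
; TakeDamage and AddHealth change Health and clamp the result between zero and MaxHealth.
; Getters expose health as a float, the health-to-maximum ratio, and an alive check.
; The event graph holds no logic, so health changes only through function calls and broadcasts no events.
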(fn `AddHealth`
  (params (Health :type Integer))
  (set `self.Health` (`KismetMathLibrary.Clamp` (+ (`self.Health`) Health) 0 (`self.MaxHealth`))))

(fn `Get Health Percentage`
  (returns (HealthPercentage :type "Float (double-precision)"))
  (return (/ (`KismetMathLibrary.Conv_IntToDouble` (`self.Health`)) (`KismetMathLibrary.Conv_IntToDouble` (`self.MaxHealth`)))))

(fn `GetHealth`
  (returns (Health :type "Float (double-precision)"))
  (return (`KismetMathLibrary.Conv_IntToDouble` (`self.Health`))))

(fn `IsAlive`
  (returns (Result :type Boolean))
  (return (> (`self.Health`) 0)))

(fn `TakeDamage`
  (params (Damage :type Integer))
  (set `self.Health` (`KismetMathLibrary.Clamp` (+ (`self.Health`) (* Damage -1)) 0 (`self.MaxHealth`))))