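; A box volume that repeatedly damages the player character while it stands inside.
; Overlap begin and end events on the Box set a flag when a Player enters or leaves.
; Tick counts down a short delay, then calls TakeDamage on the HealthComponent of player 0 and restarts the delay, rather than damaging the overlapping actor directly.
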(event `self.Box.OnComponentBeginOverlap`
  (params (OverlappedComponent :type "PrimitiveComponent Object Reference") (OtherActor :type "Actor Object Reference") (OtherComp :type "PrimitiveComponent Object Reference") (OtherBodyIndex :type Integer) (bFromSweep :type Boolean) (SweepResult :type "HitResult Structure (by ref)"))
  (cast `/Game/Blueprints/Characters/Player` OtherActor)
  (set `self.IsCharacterInVolume` true))

(event `self.Box.OnComponentEndOverlap`
  (params (OverlappedComponent :type "PrimitiveComponent Object Reference") (OtherActor :type "Actor Object Reference") (OtherComp :type "PrimitiveComponent Object Reference") (OtherBodyIndex :type Integer))
  (cast `/Game/Blueprints/Characters/Player` OtherActor)
  (set `self.IsCharacterInVolume` false))

(event `self.ReceiveTick`
  (params (DeltaSeconds :type "Float (single-precision)"))
  (if (> (`self.Delay`) 0.0)
    (set `self.Delay` (- (`self.Delay`) DeltaSeconds))
    (elif (`self.IsCharacterInVolume`)
      (bind _asplayer (cast `/Game/Blueprints/Characters/Player` (`GameplayStatics.GetPlayerCharacter` 0)))
      (`/Game/Blueprints/CharacterBaseWithComponents/HealthComponent.TakeDamage` (`/Game/Blueprints/CharacterBaseWithComponents/CharacterComponents.HealthComponent` _asplayer) 1)
      (set `self.Delay` 0.1))))

(fn `UserConstructionScript`)